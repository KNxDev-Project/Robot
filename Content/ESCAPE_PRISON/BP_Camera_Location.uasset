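; BP_Camera_Location is a trigger zone that repositions the third-person player's camera while the player is inside its Box.
; Box overlap events toggle an IN flag, and Tick then teleports the player's camera to the Arrow's world location.
; With MovableCamera set, Y instead follows the player: Arrow and capsule Y are summed and divided by CameraSpeed.
; Only location is set, and leaving the Box stops updates without restoring the camera.
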(event `self.ReceiveBeginPlay`
  (bind _asbp_third_person_character (cast `/Game/ThirdPerson/Blueprints/BP_ThirdPersonCharacter` (`GameplayStatics.GetPlayerCharacter` 0)))
  (set `self.Player` _asbp_third_person_character))

(event `self.ReceiveTick`
  (params (DeltaSeconds :type "Float (single-precision)"))
  (bind (_returnvalue_x _returnvalue_y _returnvalue_z) (`KismetMathLibrary.BreakVector` (`SceneComponent.K2_GetComponentLocation` (`self.Arrow`))))
  (bind (_returnvalue_x_2 _returnvalue_y_2) (`KismetMathLibrary.BreakVector` (`SceneComponent.K2_GetComponentLocation` (`Character.CapsuleComponent` (`self.Player`)))))
  (if (`self.IN`)
    (if (`self.MovableCamera`)
      (`SceneComponent.K2_SetWorldLocation` (`/Game/ThirdPerson/Blueprints/BP_ThirdPersonCharacter.Camera` (`self.Player`)) (`KismetMathLibrary.MakeVector` _returnvalue_x (/ (+ _returnvalue_y _returnvalue_y_2) (`self.CameraSpeed`)) _returnvalue_z) false true)
      (else
        (`SceneComponent.K2_SetWorldLocation` (`/Game/ThirdPerson/Blueprints/BP_ThirdPersonCharacter.Camera` (`self.Player`)) (`SceneComponent.K2_GetComponentLocation` (`self.Arrow`)) false true)))))

(event `self.Box.OnComponentBeginOverlap`
  (params (OverlappedComponent :type "PrimitiveComponent Object Reference") (OtherActor :type "Actor Object Reference") (OtherComp :type "PrimitiveComponent Object Reference") (OtherBodyIndex :type Integer) (bFromSweep :type Boolean) (SweepResult :type "HitResult Structure (by ref)"))
  (if (== OtherActor (`self.Player`))
    (set `self.IN` true)))

(event `self.Box.OnComponentEndOverlap`
  (params (OverlappedComponent :type "PrimitiveComponent Object Reference") (OtherActor :type "Actor Object Reference") (OtherComp :type "PrimitiveComponent Object Reference") (OtherBodyIndex :type Integer))
  (if (== OtherActor (`self.Player`))
    (set `self.IN` false)))

(fn `UserConstructionScript`)