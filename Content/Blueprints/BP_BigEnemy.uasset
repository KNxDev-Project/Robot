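; BP_BigEnemy is an enemy that catches the player on sight with a laser and forces a respawn.
; Tick alternates a Timeline between play-from-start and reverse-from-end through a FlipFlop, with updates setting the actor's yaw at a fixed downward pitch.
; PawnSensing triggers a DoOnce sequence: disable input, spawn a Niagara beam to the seen pawn, shake the camera, respawn the hero, then re-arm.
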(event `self.ReceiveBeginPlay`
  (bind _asbp_hero_character (cast `/Game/_Robot/Blueprints/Character/BP_HeroCharacter` (`GameplayStatics.GetPlayerCharacter` 0)))
  (set `self.Player` _asbp_hero_character))

(event `self.ReceiveTick`
  (params (DeltaSeconds :type "Float (single-precision)"))
  (`/Engine/EditorBlueprintResources/StandardMacros.FlipFlop`
    (:`A`
      (bind (_direction _newtrack_0) (`Timeline|Timeline` :!via `PlayFromStart` :!label _label)
        (:`Update`
          (`self.K2_SetActorRelativeRotation` (`KismetMathLibrary.MakeRotator` 0.0 -23.0 (* _newtrack_0 -166.0))))))
    (:`B`
      (goto _label :!via `ReverseFromEnd`))))

(event `self.PawnSensing.OnSeePawn`
  (params (Pawn :type "Pawn Object Reference"))
  (bind _returnvalue (`self.K2_GetActorLocation`))
  (`/Engine/EditorBlueprintResources/StandardMacros.DoOnce` false :!label _label_2
    (:`Completed`
      (`self.DisableInput` (`self.Player`) (`GameplayStatics.GetPlayerController` 0))
      (bind _returnvalue_2 (`NiagaraFunctionLibrary.SpawnSystemAtLocation` "/Game/ESCAPE_PRISON/VFX/NS_Laser.NS_Laser" _returnvalue (`self.K2_GetActorRotation`)))
      (`NiagaraComponent.SetVariableVec3` _returnvalue_2 "BeamStart" _returnvalue)
      (`NiagaraComponent.SetVariableVec3` _returnvalue_2 "BeamEnd" (`self.K2_GetActorLocation` Pawn))
      (`KismetSystemLibrary.Delay` 1.5)
      (`GameplayStatics.PlayWorldCameraShake` "/Game/Blueprints/BP_CameraShake.BP_CameraShake_C" (`self.K2_GetActorLocation`) 0.0 6000.0)
      (`KismetSystemLibrary.Delay` 1.0)
      (`/Game/_Robot/Blueprints/Character/BP_HeroCharacter.Respawn` (`self.Player`))
      (goto _label_2 :!via `Reset`))))

(fn `UserConstructionScript`)