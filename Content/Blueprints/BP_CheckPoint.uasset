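; BP_CheckPoint is a checkpoint actor that records the hero's position when its trigger box is overlapped.
; On BeginPlay it caches the first player character as a BP_HeroCharacter.
; The first box overlap passes a DoOnce and, if the overlapping actor is that player, copies the player's location and rotation into the hero's cached transform variables.
; The DoOnce precedes the player check, so any other overlapping actor also uses it up.
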(event `self.ReceiveBeginPlay`
  (bind _asbp_hero_character (cast `/Game/_Robot/Blueprints/Character/BP_HeroCharacter` (`GameplayStatics.GetPlayerCharacter` 0)))
  (set `self.Player` _asbp_hero_character))

(event `self.Box.OnComponentBeginOverlap`
  (params (OverlappedComponent :type "PrimitiveComponent Object Reference") (OtherActor :type "Actor Object Reference") (OtherComp :type "PrimitiveComponent Object Reference") (OtherBodyIndex :type Integer) (bFromSweep :type Boolean) (SweepResult :type "HitResult Structure (by ref)"))
  (bind _player (`self.Player`))
  (`/Engine/EditorBlueprintResources/StandardMacros.DoOnce` false
    (:`Completed`
      (if (== OtherActor (`self.Player`))
        (set `/Game/_Robot/Blueprints/Character/BP_HeroCharacter.CashedLocation` (`self.K2_GetActorLocation` _player) _player)
        (set `/Game/_Robot/Blueprints/Character/BP_HeroCharacter.CashedRotation` (`self.K2_GetActorRotation` _player) _player)))))

(fn `UserConstructionScript`)