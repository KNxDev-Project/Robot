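; Player hero character that spawns its own camera actor, interacts with nearby objects and supports ragdoll death and respawn.
; On BeginPlay it spawns BP_Camera, links itself as its Hero and makes it the view target.
; A throttled Tick sphere-traces for BPI_Interactable actors, sending focus or defocus; E interacts when allowed.
; Death disables input and ragdolls the mesh; Respawn reattaches it, restores input and teleports to a cached transform.
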(event `self.ReceiveBeginPlay`
  (bind _returnvalue (`|SpawnActorFromClass` "/Game/_Robot/Blueprints/Character/BP_Camera.BP_Camera_C" (`KismetMathLibrary.MakeTransform` (`self.K2_GetActorLocation`)) "AdjustIfPossibleButAlwaysSpawn" "MultiplyWithRoot" null null))
  (bind _output_get (set `self.Camera` _returnvalue))
  (set `/Game/_Robot/Blueprints/Character/BP_Camera.Hero` self _output_get)
  (`PlayerController.SetViewTargetWithBlend` (cast `PlayerController` (`self.GetController`) :!pure true) (`self.Camera`) 0.0 "VTBlend_Linear" 0.0 false)
  (`self.SetActorTickEnabled` (`self.Camera`) true))

(event `Key|E`
  (params (Key :type "Key Structure"))
  (:`Pressed`
    (bind _caninteract (message `/Game/_Robot/Blueprints/Interaction/BPI_Interactable.CanInteract` (`self.CurrentInteractable`) self))
    (if _caninteract
      (message `/Game/_Robot/Blueprints/Interaction/BPI_Interactable.Interact` (`self.CurrentInteractable`) self))))

(event `self.ReceiveTick`
  (params (DeltaSeconds :type "Float (single-precision)"))
  (bind _returnvalue (`self.K2_GetActorLocation`))
  (bind _currentinteractable (`self.CurrentInteractable`))
  (bind (_outhit _returnvalue_2) (`KismetSystemLibrary.SphereTraceSingle` :`Start` _returnvalue :`End` (+ _returnvalue (0.0 0.0 0.1)) :`Radius` (`self.InteractRadius`) :`TraceChannel` "TraceTypeQuery3" :`DrawTime` 0.1))
  (if (and (`KismetSystemLibrary.DoesImplementInterface` (`.HitActor` (`GameplayStatics.BreakHitResult` _outhit)) "/Game/_Robot/Blueprints/Interaction/BPI_Interactable.BPI_Interactable_C") _returnvalue_2)
    (set `self.CurrentInteractable` (`.HitActor` (`GameplayStatics.BreakHitResult` _outhit)))
    (message `/Game/_Robot/Blueprints/Interaction/BPI_Interactable.Focus` _currentinteractable self)
    (else
      (message `/Game/_Robot/Blueprints/Interaction/BPI_Interactable.Defocus` _currentinteractable self)
      (set `self.CurrentInteractable` null))))

(fn `Death`
  (`self.DisableInput` (`GameplayStatics.GetPlayerController` 0))
  (`PrimitiveComponent.SetSimulatePhysics` (`self.Mesh`) true))

(fn `Respawn`
  (`PrimitiveComponent.SetSimulatePhysics` (`self.Mesh`) false)
  (`SceneComponent.K2_AttachToComponent` (`self.Mesh`) (`self.CapsuleComponent`) "None" "KeepRelative" "KeepRelative" "KeepRelative" true)
  (`SceneComponent.K2_SetRelativeLocationAndRotation` (`self.Mesh`) (0.0 0.0 -95.0) (struct :`Yaw` -90.0) false true)
  (`self.EnableInput` (`GameplayStatics.GetPlayerController` 0))
  (`self.K2_TeleportTo` (`self.CashedLocation`) (`self.CashedRotation`)))

(fn `UserConstructionScript`)