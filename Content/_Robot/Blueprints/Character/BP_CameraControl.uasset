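; BP_CameraControl is a trigger volume that takes over the hero's camera while the character is inside its box.
; On begin overlap it calls FocusOn on the BP_HeroCharacter camera with a lerp time, actor-relative destination and spring arm and camera overrides or defaults.
; End overlap calls ResetCamera.
; The construction script adds an arrow and a child BP_Camera configured with the same transforms and arm length, mirroring the target shot.
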(event `self.Box.OnComponentBeginOverlap`
  (params (OverlappedComponent :type "PrimitiveComponent Object Reference") (OtherActor :type "Actor Object Reference") (OtherComp :type "PrimitiveComponent Object Reference") (OtherBodyIndex :type Integer) (bFromSweep :type Boolean) (SweepResult :type "HitResult Structure (by ref)"))
  (bind _returnvalue (`self.GetTransform`))
  (bind (_asbp_hero_character _bsuccess) (cast `/Game/_Robot/Blueprints/Character/BP_HeroCharacter` OtherActor :!pure true))
  (bind (_cameraactortransform_location _cameraactortransform_rotation) (`KismetMathLibrary.BreakTransform` (`self.CameraActorTransform`)))
  (bind (_springarmrelativetransform_location _springarmrelativetransform_rotation) (`KismetMathLibrary.BreakTransform` (`self.SpringArmRelativeTransform`)))
  (bind (_camerarelativetransform_location _camerarelativetransform_rotation) (`KismetMathLibrary.BreakTransform` (`self.CameraRelativeTransform`)))
  (if _bsuccess
    (bind _camera (`/Game/_Robot/Blueprints/Character/BP_HeroCharacter.Camera` _asbp_hero_character)
      (:`then`
        (`/Game/_Robot/Blueprints/Character/BP_Camera.FocusOn` _camera (`self.LerpTime`) (`KismetMathLibrary.TransformLocation` _returnvalue _cameraactortransform_location) (`KismetMathLibrary.TransformRotation` _returnvalue _cameraactortransform_rotation) _springarmrelativetransform_rotation (`self.UseDefaultSpringArmRelativeRotation`) (`self.TargetArmLength`) (`self.UseDefaultTargetArmLength`) _camerarelativetransform_rotation (`self.UseDefaultCameraRelativeRotation`)))
      (:`else`))))

(event `self.Box.OnComponentEndOverlap`
  (params (OverlappedComponent :type "PrimitiveComponent Object Reference") (OtherActor :type "Actor Object Reference") (OtherComp :type "PrimitiveComponent Object Reference") (OtherBodyIndex :type Integer))
  (bind (_asbp_hero_character _bsuccess) (cast `/Game/_Robot/Blueprints/Character/BP_HeroCharacter` OtherActor :!pure true))
  (if _bsuccess
    (bind _camera (`/Game/_Robot/Blueprints/Character/BP_HeroCharacter.Camera` _asbp_hero_character)
      (:`then`
        (`/Game/_Robot/Blueprints/Character/BP_Camera.ResetCamera` _camera))
      (:`else`))))

(fn `UserConstructionScript`
  (bind (_cameraactortransform_location _cameraactortransform_rotation _cameraactortransform_scale) (`KismetMathLibrary.BreakTransform` (`self.CameraActorTransform`)))
  (bind (_cameraactortransform_location_2 _cameraactortransform_rotation_2) (`KismetMathLibrary.BreakTransform` (`self.CameraActorTransform`)))
  (`AddComponent|NODE_AddArrowComponent-0` :`RelativeTransform` (`KismetMathLibrary.MakeTransform` _cameraactortransform_location _cameraactortransform_rotation _cameraactortransform_scale))
  (bind _returnvalue (`AddComponent|NODE_AddChildActorComponent-0` :`RelativeTransform` (`KismetMathLibrary.MakeTransform` _cameraactortransform_location_2 _cameraactortransform_rotation_2)))
  (bind _asbp_camera (cast `/Game/_Robot/Blueprints/Character/BP_Camera` (`ChildActorComponent.ChildActor` _returnvalue)))
  (bind _springarm (`/Game/_Robot/Blueprints/Character/BP_Camera.SpringArm` _asbp_camera))
  (`SceneComponent.K2_SetRelativeTransform` _springarm (`self.SpringArmRelativeTransform`) false false)
  (set `SpringArmComponent.TargetArmLength` (`self.TargetArmLength`) _springarm)
  (`SceneComponent.K2_SetRelativeTransform` (`/Game/_Robot/Blueprints/Character/BP_Camera.Camera` _asbp_camera) (`self.CameraRelativeTransform`) false false))