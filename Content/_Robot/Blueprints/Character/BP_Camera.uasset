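; Hero camera rig with a spring arm that follows the Hero on Tick and can blend to a fixed focus view.
; FocusOn stops following and uses a timeline to lerp location, rotation, arm length and relative rotations to given or default values.
; ResetCamera resumes Tick and blends back to the Hero and the defaults saved at construction.
; ResetCamera applies LerpTime to ChangeLocationTimeline, although it plays ResetCameraTimeline.
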(event `self.ReceiveTick`
  (params (DeltaSeconds :type "Float (single-precision)"))
  (`self.Hero`
    (:`then`
      (`self.K2_SetActorLocation` (`KismetMathLibrary.VInterpTo` (`self.K2_GetActorLocation`) (`self.K2_GetActorLocation` (`self.Hero`)) DeltaSeconds 70.0)))
    (:`else`
      (`self.SetActorTickEnabled` false))))

(fn `FocusOn`
  (params (LerpTime :type "Float (double-precision)" :default 0.5) (DestinationLocation :type "Vector Structure") (DestinationRotation :type "Rotator Structure") (SpringArmRelativeRotation :type "Rotator Structure" :default (struct :`Pitch` -10.0)) (UseDefaultSpringArmRelativeRotation :type Boolean :default true) (TargetArmLength :type "Float (double-precision)" :default 520.0) (UseDefaultTargetArmLength :type Boolean :default true) (CameraRelativeRotation :type "Rotator Structure" :default (struct :`Pitch` 10.0)) (UseDefaultCameraRelativeRotation :type Boolean :default true))
  (`TimelineComponent.Stop` (`self.ResetCameraTimeline`))
  (`|ExecutionSequence`
    (:`then_0`
      (`TimelineComponent.SetPlayRate` (`self.ChangeLocationTimeline`) (/ 1.0 (`local.LerpTime`)))
      (set `self.FocusStartLocation` (`self.K2_GetActorLocation`))
      (set `self.FocusStartRotation` (`self.K2_GetActorRotation`))
      (set `self.FocusStartSpringArmRelativeRotation` (`SceneComponent.RelativeRotation` (`self.SpringArm`)))
      (set `self.FocusStartTargetArmLength` (`SpringArmComponent.TargetArmLength` (`self.SpringArm`)))
      (set `self.FocusStartCameraRelativeRotation` (`SceneComponent.RelativeRotation` (`self.Camera`))))
    (:`then_1`
      (set `self.FocusDestinationLocation` (`local.DestinationLocation`))
      (set `self.FocusDestinationRotation` (`local.DestinationRotation`))
      (set `self.FocusDestinationSpringArmRelativeRotation` (select `bool` (`local.UseDefaultSpringArmRelativeRotation`) :`false` (`local.SpringArmRelativeRotation`) :`true` (`self.DefaultSpringArmRelativeRotation`)))
      (set `self.FocusDestinationTargetArmLength` (select `bool` (`local.UseDefaultTargetArmLength`) :`false` (`local.TargetArmLength`) :`true` (`self.DefaultSpringArmTargetArmLength`) :!type "Float (single-precision)"))
      (set `self.FocusDestinationCameraRelativeRotation` (select `bool` (`local.UseDefaultCameraRelativeRotation`) :`false` (`local.CameraRelativeRotation`) :`true` (`self.DefaultCameraRelativeRotation`))))
    (:`then_2`
      (`self.SetActorTickEnabled` false)
      (`TimelineComponent.PlayFromStart` (`self.ChangeLocationTimeline`)))))

(fn `ResetCamera`
  (params (LerpTime :type "Float (single-precision)" :default 0.5))
  (`TimelineComponent.Stop` (`self.ChangeLocationTimeline`))
  (`|ExecutionSequence`
    (:`then_0`
      (`TimelineComponent.SetPlayRate` (`self.ChangeLocationTimeline`) (/ 1.0 (`local.LerpTime`)))
      (set `self.FocusStartLocation` (`self.K2_GetActorLocation`))
      (set `self.FocusStartRotation` (`self.K2_GetActorRotation`))
      (set `self.FocusStartSpringArmRelativeRotation` (`SceneComponent.RelativeRotation` (`self.SpringArm`)))
      (set `self.FocusStartTargetArmLength` (`SpringArmComponent.TargetArmLength` (`self.SpringArm`)))
      (set `self.FocusStartCameraRelativeRotation` (`SceneComponent.RelativeRotation` (`self.Camera`))))
    (:`then_1`
      (set `self.FocusDestinationRotation` (struct))
      (set `self.FocusDestinationSpringArmRelativeRotation` (`self.DefaultSpringArmRelativeRotation`))
      (set `self.FocusDestinationTargetArmLength` (`self.DefaultSpringArmTargetArmLength`))
      (set `self.FocusDestinationCameraRelativeRotation` (`self.DefaultCameraRelativeRotation`)))
    (:`then_2`
      (`self.SetActorTickEnabled` true)
      (`TimelineComponent.PlayFromStart` (`self.ResetCameraTimeline`)))))

(fn `UserConstructionScript`
  (set `self.DefaultSpringArmRelativeRotation` (`SceneComponent.RelativeRotation` (`self.SpringArm`)))
  (set `self.DefaultSpringArmTargetArmLength` (`SpringArmComponent.TargetArmLength` (`self.SpringArm`)))
  (set `self.DefaultCameraRelativeRotation` (`SceneComponent.RelativeRotation` (`self.Camera`))))