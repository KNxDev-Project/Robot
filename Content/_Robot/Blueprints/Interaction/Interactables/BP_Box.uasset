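; BP_Box is an interactable box that shows a text prompt while focused.
; Focus and Defocus show and hide its TextRender, with Focus suppressed while an interaction is pending.
; Interact toggles the PendingInteraction flag and hides the prompt when an interaction begins; no further box behavior is implemented.
; CanInteract always returns true, regardless of the interacter.
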(event `/Game/_Robot/Blueprints/Interaction/BPI_Interactable.Interact`
  (params (Interacter :type "Actor Object Reference"))
  (if (`self.PendingInteraction`)
    (set `self.PendingInteraction` false)
    (else
      (set `self.PendingInteraction` true) ; Begin interaction
      (`self.Defocus` null))))

(event `/Game/_Robot/Blueprints/Interaction/BPI_Interactable.Focus`
  (params (Interacter :type "Actor Object Reference"))
  (if (not (`self.PendingInteraction`))
    (`SceneComponent.SetHiddenInGame` (`self.TextRender`) false false)))

(event `/Game/_Robot/Blueprints/Interaction/BPI_Interactable.Defocus`
  (params (Interacter :type "Actor Object Reference"))
  (`SceneComponent.SetHiddenInGame` (`self.TextRender`) true false))

(fn `CanInteract`
  (params (Interacter :type "Actor Object Reference"))
  (returns (CanInteract :type Boolean))
  (return true))

(fn `UserConstructionScript`)